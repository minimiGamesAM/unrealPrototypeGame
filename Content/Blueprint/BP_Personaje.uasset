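; Player character with walk, trot and run modes plus a toggle between follow and tactical cameras.
; Movement modes scale axis input, and running also raises max walk speed.
; In tactical mode, zoom cycles three camera anchors through a timeline lerp, and another input steps the view through BP_EnemigoAI actors and back to the player.
; IntercambioTacticalCam blends the view target and repoints the camera references, so zoom acts on the viewed character.
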(event `self.ReceiveBeginPlay`
  ;[0.3193 1 0.2638] Inicializacion
  (set `self.TacticalCameraAMover` (`self.CameraTactica`))
  (set `self.TacticalCameraAMoverAPos0` (`self.CameraPos_0`))
  (set `self.TacticalCameraAMoverAPos1` (`self.CameraPos_1`))
  (set `self.TacticalCameraAMoverAPos2` (`self.CameraPos_2`)))

(event `InputAction|TacticalCameraModo`
  (params (Key :type "Key Structure"))
  ;[0.325 0.3963 1] Tactical Camera Modo
  (:`Pressed`
    (`/Engine/EditorBlueprintResources/StandardMacros.FlipFlop`
      (:`A`
        (`ActorComponent.Activate` (`self.CameraTactica`) false)
        (`ActorComponent.Deactivate` (`self.CameraSeguidora`))
        (set `SpringArmComponent.bDoCollisionTest` false (`self.SpringArm`))
        (set `self.TaticalCameraModoOn` true))
      (:`B`
        (`self.IntercambioTacticalCam` null)
        (`ActorComponent.Activate` (`self.CameraSeguidora`) false)
        (`ActorComponent.Deactivate` (`self.CameraTactica`))
        (set `SpringArmComponent.bDoCollisionTest` true (`self.SpringArm`))
        (set `self.TaticalCameraModoOn` false)))))

(event `InputAction|Caminar`
  (params (Key :type "Key Structure"))
  ;[0.1582 1 0.2685] Caminar Correr
  (:`Pressed`
    (`/Engine/EditorBlueprintResources/StandardMacros.FlipFlop`
      (:`A`
        (set `self.MovimientoModo` "NewEnumerator1"))
      (:`B`
        (set `self.MovimientoModo` "NewEnumerator0")))))

(event `InputAction|Correr`
  (params (Key :type "Key Structure"))
  (bind _charactermovement (`self.CharacterMovement`))
  ;[0.1582 1 0.2685] Caminar Correr
  (:`Pressed`
    (`/Engine/EditorBlueprintResources/StandardMacros.FlipFlop`
      (:`A`
        (set `self.MovimientoModo` "NewEnumerator2")
        (set `CharacterMovementComponent.MaxWalkSpeed` 800.0 _charactermovement))
      (:`B`
        (set `self.MovimientoModo` "NewEnumerator0")
        (set `CharacterMovementComponent.MaxWalkSpeed` 450.0 _charactermovement)))))

(event `InputAxis|MoveForward`
  (params (AxisValue :type "Float (single-precision)"))
  (switch `/Game/EnemyAI/EnumMovimientoMode` (`self.MovimientoModo`)
    (:`NewEnumerator0`
      (set `self.MovimientoRacionAdelante` AxisValue))
    (:`NewEnumerator1`
      (set `self.MovimientoRacionAdelante` (* AxisValue (`self.CaminadoModificador`))))
    (:`NewEnumerator2`
      (set `self.MovimientoRacionAdelante` (* AxisValue (`self.CorrerModificador`)))))
  (`self.MoveForward` (`self.MovimientoRacionAdelante`)))

(event `InputAction|TacticalCameraZoom`
  (params (Key :type "Key Structure"))
  ;[1 0.5001 0.2085] Tactical camara zoom
  (:`Pressed`
    (if (`self.TaticalCameraModoOn`)
      (`|MultiGate` false true
        (:`Out 0`
          (set `self.TacticalCameraPosicion` (`SceneComponent.RelativeLocation` (`self.TacticalCameraAMoverAPos1`)))
          (bind (_direction _conductor) (`Timeline|Timeline_0` :!label _label)
            (:`Update`
              (`SceneComponent.K2_SetRelativeLocation` (`self.TacticalCameraAMover`) (`KismetMathLibrary.VLerp` (`SceneComponent.RelativeLocation` (`self.TacticalCameraAMover`)) (`self.TacticalCameraPosicion`) _conductor) false false))))
        (:`Out 1`
          (set `self.TacticalCameraPosicion` (`SceneComponent.RelativeLocation` (`self.TacticalCameraAMoverAPos2`)))
          (goto _label :!via `PlayFromStart`))
        (:`Out 2`
          (set `self.TacticalCameraPosicion` (`SceneComponent.RelativeLocation` (`self.TacticalCameraAMoverAPos0`)))
          (goto _label :!via `PlayFromStart`))))))

(event `InputAxis|MoveRight`
  (params (AxisValue :type "Float (single-precision)"))
  (switch `/Game/EnemyAI/EnumMovimientoMode` (`self.MovimientoModo`)
    (:`NewEnumerator0`
      (set `self.MoviemientoRacioDerecha` AxisValue))
    (:`NewEnumerator1`
      (set `self.MoviemientoRacioDerecha` (* AxisValue (`self.CaminadoModificador`))))
    (:`NewEnumerator2`
      (set `self.MoviemientoRacioDerecha` (* AxisValue (`self.CorrerModificador`)))))
  (`self.MoveRight` (`self.MoviemientoRacioDerecha`)))

(event `InputAction|IntercambioEnemigoAICamara`
  (params (Key :type "Key Structure"))
  (bind _objetivosdevistas (`self.ObjetivosDeVistas`))
  (bind _objetivosdevistas_2 (`self.ObjetivosDeVistas`))
  (bind _tacticalcamaraindex (`self.TacticalCamaraIndex`))
  (:`Pressed`
    (if (and (`self.TaticalCameraModoOn`) (`self.TacCamIntercambioCompletado`))
      (set `self.TacCamIntercambioCompletado` false)
      (`KismetArrayLibrary.Array_Clear` _objetivosdevistas)
      (`KismetArrayLibrary.Array_Resize` _objetivosdevistas)
      (bind _outactors (`GameplayStatics.GetAllActorsOfClass` "/Game/Blueprint/BP_EnemigoAI.BP_EnemigoAI_C"))
      (if (> (`KismetArrayLibrary.Array_Length` _outactors) 0)
        (for _array_element _outactors
          (`KismetArrayLibrary.Array_Add` _objetivosdevistas_2 _array_element))
        (`KismetArrayLibrary.Array_Add` _objetivosdevistas_2 (`GameplayStatics.GetPlayerCharacter` 0))
        (if (< _tacticalcamaraindex (- (`KismetArrayLibrary.Array_Length` (`self.ObjetivosDeVistas`)) 1))
          (bind _asbp_enemigo_ai (cast `/Game/Blueprint/BP_EnemigoAI` (`|GetArrayItem` (`self.ObjetivosDeVistas`) _tacticalcamaraindex)))
          (`self.IntercambioTacticalCam` _asbp_enemigo_ai)
          (set `self.TacticalCamaraIndex` (+ (`self.TacticalCamaraIndex`) 1))
          (else
            (`self.IntercambioTacticalCam` null)
            (set `self.TacticalCamaraIndex` 0)))
        (`KismetSystemLibrary.Delay` 1.0)
        (set `self.TacCamIntercambioCompletado` true)))))

(fn `IntercambioTacticalCam`
  (params (EnemigoAI :type "/Game/Blueprint/BP_EnemigoAI Object Reference"))
  (bind _returnvalue (`GameplayStatics.GetPlayerController` 0))
  (if (!= EnemigoAI null)
    (set `self.TacticalCameraAMover` (`/Game/Blueprint/BP_EnemigoAI.CameraTactica` EnemigoAI))
    (set `self.TacticalCameraAMoverAPos0` (`/Game/Blueprint/BP_EnemigoAI.CameraPos_0` EnemigoAI))
    (set `self.TacticalCameraAMoverAPos1` (`/Game/Blueprint/BP_EnemigoAI.CameraPos_1` EnemigoAI))
    (set `self.TacticalCameraAMoverAPos2` (`/Game/Blueprint/BP_EnemigoAI.CameraPos_2` EnemigoAI))
    (`PlayerController.SetViewTargetWithBlend` _returnvalue EnemigoAI 1.0 "VTBlend_Cubic" 3.0 false)
    (else
      (set `self.TacticalCameraAMover` (`self.CameraTactica`))
      (set `self.TacticalCameraAMoverAPos0` (`self.CameraPos_0`))
      (set `self.TacticalCameraAMoverAPos1` (`self.CameraPos_1`))
      (set `self.TacticalCameraAMoverAPos2` (`self.CameraPos_2`))
      (`PlayerController.SetViewTargetWithBlend` _returnvalue self 1.0 "VTBlend_Cubic" 3.0 false)))
  (return))

(fn `UserConstructionScript`)